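; Car actor whose doors, hood and boot can animate into place, as in an assembly sequence, while the car creeps forward.
; Construction script hides those parts, then snaps any flagged by Close booleans to hard-coded fitted transforms and unhides them.
; AssembleCars reveals meshes matching a component tag and lerps them from current to fitted transforms via the CarAssemble timeline.
; Tick applies a fixed per-frame local Y offset while Move is set.
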(event `AssembleCars`
  (params (ComTag :type Name))
  (`KismetArrayLibrary.Array_Clear` (`self.AnimatedTransform`))
  (`KismetArrayLibrary.Array_Clear` (`self.AnimatedObject`))
  (for _array_element (`self.K2_GetComponentsByClass` self "/Script/Engine.StaticMeshComponent")
    (if (`ActorComponent.ComponentHasTag` _array_element ComTag)
      (`KismetArrayLibrary.Array_Add` (`self.AnimatedObject`) _array_element)
      (`KismetArrayLibrary.Array_Add` (`self.AnimatedTransform`) (`SceneComponent.GetRelativeTransform` _array_element))
      (`SceneComponent.SetHiddenInGame` _array_element false false)
      (bind (_direction _timea) (`Timeline|CarAssemble` :!via `PlayFromStart`)
        (:`Update`
          (for (_array_element_2 _array_index) (`self.AnimatedObject`)
            (bind _returnindex (`self.SetSelectIndex` _array_element_2))
            (set `self.SelectIndex` _returnindex)
            (`SceneComponent.K2_SetRelativeTransform` _array_element_2 (`KismetMathLibrary.TLerp` (`|GetArrayItem` (`self.AnimatedTransform`) _array_index) (select `int` (`self.SelectIndex`) :`0` (`KismetMathLibrary.MakeTransform` (-71.0 -54.261162 63.832382) (struct) (1.0 1.0 1.0)) :`1` (`KismetMathLibrary.MakeTransform` (71.0 -54.261162 63.832382) (struct) (-1.0 1.0 1.0)) :`2` (`KismetMathLibrary.MakeTransform` (-71.0 36.849506 67.259232) (struct) (1.0 1.0 1.0)) :`3` (`KismetMathLibrary.MakeTransform` (71.0 36.849506 67.259232) (struct) (-1.0 1.0 1.0)) :`4` (`KismetMathLibrary.MakeTransform` (0.0 -71.342026 94.792213) (struct) (1.0 1.0 1.0)) :`5` (`KismetMathLibrary.MakeTransform` (0.0 141.946716 139.415207) (struct) (1.0 1.0 1.0)) :!type "Transform Structure") _timea) false false)))))))

(event `self.ReceiveTick`
  (params (DeltaSeconds :type "Float (single-precision)"))
  (`self.AutoMove` (0.0 0.5 0.0)))

(fn `AutoMove`
  (params (DeltaLocation :type "Vector Structure" :default (0.0 0.5 0.0)))
  (if (`self.Move?`)
    (`self.K2_AddActorLocalOffset` DeltaLocation)))

(fn `CloseDoor`
  (`|ExecutionSequence`
    (:`then_0`
      (if (`self.Close_FDoor`)
        (`SceneComponent.K2_SetRelativeTransform` (`self.FrontDoor_01`) (`KismetMathLibrary.MakeTransform` (-71.0 -54.261162 63.832382)) false false)
        (`SceneComponent.K2_SetRelativeTransform` (`self.FrontDoor_02`) (`KismetMathLibrary.MakeTransform` (71.0 -54.261162 63.832382) (struct) (-1.0 1.0 1.0)) false false)
        (`SceneComponent.SetHiddenInGame` (`self.FrontDoor_01`) false false)
        (`SceneComponent.SetHiddenInGame` (`self.FrontDoor_01`) false false)))
    (:`then_1`
      (if (`self.Close_BDoor`)
        (`SceneComponent.K2_SetRelativeTransform` (`self.RearDoor_01`) (`KismetMathLibrary.MakeTransform` (-71.0 36.849506 67.259232)) false false)
        (`SceneComponent.K2_SetRelativeTransform` (`self.RearDoor_02`) (`KismetMathLibrary.MakeTransform` (71.0 36.849506 67.259232) (struct) (-1.0 1.0 1.0)) false false)
        (`SceneComponent.SetHiddenInGame` (`self.RearDoor_01`) false false)
        (`SceneComponent.SetHiddenInGame` (`self.RearDoor_02`) false false)))
    (:`then_2`
      (if (`self.Close_Hood`)
        (`SceneComponent.K2_SetRelativeTransform` (`self.Hood`) (`KismetMathLibrary.MakeTransform` (-7.6e-05 -71.342026 94.792213)) false false)
        (`SceneComponent.SetHiddenInGame` (`self.Hood`) false false)))
    (:`then_3`
      (if (`self.Close_Boot`)
        (`SceneComponent.K2_SetRelativeTransform` (`self.Boot`) (`KismetMathLibrary.MakeTransform` (0.0 141.946716 139.415207)) false false)
        (`SceneComponent.SetHiddenInGame` (`self.Boot`) false false)))))

(fn `HidderMesh`
  (`SceneComponent.SetHiddenInGame` (`self.RearDoor_01`) true false)
  (`SceneComponent.SetHiddenInGame` (`self.RearDoor_02`) true false)
  (`SceneComponent.SetHiddenInGame` (`self.FrontDoor_01`) true false)
  (`SceneComponent.SetHiddenInGame` (`self.FrontDoor_02`) true false)
  (`SceneComponent.SetHiddenInGame` (`self.Boot`) true false)
  (`SceneComponent.SetHiddenInGame` (`self.Hood`) true false))

(fn `SetSelectIndex`
  (params (StaticMeshCom :type "StaticMeshComponent Object Reference"))
  (returns (ReturnIndex :type Integer))
  (if (== StaticMeshCom (`self.FrontDoor_01`))
    (return 0)
    (elif (== StaticMeshCom (`self.FrontDoor_02`))
      (return 1)
      (elif (== StaticMeshCom (`self.RearDoor_01`))
        (return 2)
        (elif (== StaticMeshCom (`self.RearDoor_02`))
          (return 3)
          (elif (== StaticMeshCom (`self.Hood`))
            (return 4)
            (elif (== StaticMeshCom (`self.Boot`))
              (return 5)
              (else
                (return -1)))))))))

(fn `UserConstructionScript`
  (`self.HidderMesh`)
  (`self.CloseDoor`))