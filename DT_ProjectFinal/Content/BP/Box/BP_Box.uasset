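; BP_Box is a box actor whose color and size come from its BoxConfig settings.
; On BeginPlay it assigns a cube mesh, creates a dynamic instance of M_Box and sets its BaseColor by looking up the configured color type in the MColor map.
; It then applies the configured size as the mesh's world scale.
; The overlap event and construction script are empty.
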(event `self.ReceiveBeginPlay`
  (bind _boxconfig_boxsize (break `/Game/BP/BoxData/ST_BoxInfo` (`self.BoxConfig`)))
  (`StaticMeshComponent.SetStaticMesh` (`self.StaticMesh`) "/Game/StarterContent/Shapes/Shape_Cube.Shape_Cube")
  (bind _returnvalue (`PrimitiveComponent.CreateDynamicMaterialInstance` (`self.StaticMesh`) 0 "/Game/BP/Box/M_Box.M_Box" "None"))
  (bind _output_get (set `self.DynamicBoxMatarial` _returnvalue))
  (`MaterialInstanceDynamic.SetVectorParameterValue` _output_get "BaseColor" (`BlueprintMapLibrary.Map_Find` (`self.mColor`) (`.BoxColorType_47_012133E841E581913E8470A912192017` (break `/Game/BP/BoxData/ST_BoxInfo` (`self.BoxConfig`)))))
  (`SceneComponent.SetWorldScale3D` (`self.StaticMesh`) _boxconfig_boxsize))

(fn `UserConstructionScript`)