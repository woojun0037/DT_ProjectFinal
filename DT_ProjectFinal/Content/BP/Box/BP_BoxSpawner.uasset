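; BP_BoxSpawner spawns boxes onto a spline path and moves them along it like a conveyor.
; A looping timer from BeginPlay spawns a box using random SpawnData at the first BP_MySpline's start, adding it to BoxList.
; Tick teleports each box with spline movement active along the SplineTransfom spline.
; Each frame derives distance from the box's location and advances it by SpeedOnSpline, scaled by delta time.
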(event `Spawn`
  (bind (_boxtypeinfo _boxbpclass) (break `/Game/BP/BoxData/ST_BoxSpawnData` (`KismetArrayLibrary.Array_Random` (`self.SpawnData`))))
  (bind _outactors (`GameplayStatics.GetAllActorsOfClass` "/Game/BP/Spline/BP_MySpline.BP_MySpline_C"))
  (if (`KismetArrayLibrary.Array_IsNotEmpty` _outactors)
    (bind _output (`|GetArrayItem` _outactors))
    (bind _returnvalue (`|SpawnActorFromClass` _boxbpclass (`SplineComponent.GetTransformAtSplinePoint` (`/Game/BP/Spline/BP_MySpline.PathSpline` _output) 0 "World" false) "Undefined" "MultiplyWithRoot" self _boxtypeinfo _output null))
    (bind _output_get (set `self.BP_Box` _returnvalue))
    ; 중복 인덱스 방지
    (`KismetArrayLibrary.Array_AddUnique` (`self.BoxList`) _output_get)))

(event `self.ReceiveBeginPlay`
  (`KismetSystemLibrary.K2_SetTimerDelegate` (delegate `Spawn`) 1.5 true))

(event `self.ReceiveTick`
  (params (DeltaSeconds :type "Float (single-precision)"))
  (bind _pathspline (`/Game/BP/Spline/BP_MySpline.PathSpline` (`self.SplineTransfom`)))
  (for _array_element (`self.BoxList`)
    (if (`/Game/BP/Box/BP_Box.bSplineMovementAcive` _array_element)
      (`self.K2_SetActorTransform` _array_element (`SplineComponent.GetTransformAtDistanceAlongSpline` _pathspline (+ (`SplineComponent.GetDistanceAlongSplineAtLocation` _pathspline (`self.K2_GetActorLocation` _array_element) "World") (* DeltaSeconds (`self.Speed On Spline`))) "World" false) false true))))

(fn `UserConstructionScript`)