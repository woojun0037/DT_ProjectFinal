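; Robot arm actor that finds BP_Box actors, picks them up and carries them to a drop position.
; An event-driven state machine starts with a looping timer sphere search, then moves a Control Rig end control toward the found box on Tick.
; Box overlap attaches it to a mesh socket, stops its spline movement and targets DropPos.
; DropCollison overlap detaches it, tags it with the arm's name and resumes searching.
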(event `self.ControlRig.OnPreInitializeDelegate`
  (params (Component :type "ControlRigComponent Object Reference"))
  ; Initailize and Mapped
  (`ControlRigComponent.AddMappedCompleteSkeletalMesh` (`self.ControlRig`) (`self.SkeletalMesh`) "Output"))

(event `self.DropCollison.OnComponentBeginOverlap`
  (params (OverlappedComponent :type "PrimitiveComponent Object Reference") (OtherActor :type "Actor Object Reference") (OtherComp :type "PrimitiveComponent Object Reference") (OtherBodyIndex :type Integer) (bFromSweep :type Boolean) (SweepResult :type "HitResult Structure (by ref)"))
  ; Overlap Event
  (if (== OtherActor (`self.BP_Box`))
    (`self.Enter_StateDroppingBox`)))

(event `self.Box.OnComponentBeginOverlap`
  (params (OverlappedComponent :type "PrimitiveComponent Object Reference") (OtherActor :type "Actor Object Reference") (OtherComp :type "PrimitiveComponent Object Reference") (OtherBodyIndex :type Integer) (bFromSweep :type Boolean) (SweepResult :type "HitResult Structure (by ref)"))
  ; Overlap Event
  (if (== OtherActor (`self.BP_Box`))
    (`self.EnterState_PickUpBox`)))

(event `self.ReceiveBeginPlay`
  ; Evenet BeginPlay
  (`self.EnterState_Idle`))

(event `self.ReceiveTick`
  (params (DeltaSeconds :type "Float (single-precision)"))
  ; Event Tick
  (switch `/Game/BP/ControlRig/E_RobotArmState` (`self.CurrentArmState`)
    (:`NewEnumerator2`
      (`self.EnterState_MovingToTarget`))))

(event `EnterState_Idle`
  ; Idle State
  (set `self.CurrentArmState` "NewEnumerator0")
  (`KismetSystemLibrary.PrintString` "Robot Arm : Idling")
  (`self.EnterState_SearchingBox`))

(event `EnterState_SearchingBox`
  ; Searching Box State
  (set `self.CurrentArmState` "NewEnumerator1")
  (bind _returnvalue (`ControlRigComponent.GetControlOffset` (`self.ControlRig`) "Robot1_End" "WorldSpace"))
  (`ControlRigComponent.SetControlTransform` (`self.ControlRig`) "Robot1_End" _returnvalue "WorldSpace")
  (`|ExecutionSequence`
    (:`then_0`
      (`KismetSystemLibrary.K2_ClearAndInvalidateTimerHandle` (`self.StateTimerHandle`)))
    (:`then_1`
      (bind _returnvalue_2 (`KismetSystemLibrary.K2_SetTimerDelegate` (delegate `StartCheckBox`) 0.1 true))
      (set `self.StateTimerHandle` _returnvalue_2))))

(event `StartCheckBox`
  (bind _searchradius (`self.SearchRadius`))
  (bind _returnvalue (`SceneComponent.K2_GetComponentLocation` (`self.ShereOverlap`)))
  ; Searching Box State
  (`KismetSystemLibrary.DrawDebugSphere` _returnvalue _searchradius 12 (struct :`R` 1.0 :`G` 0.010513 :`B` 0.012083 :`A` 1.0) 0.5 2.0)
  (bind _outactors (`KismetSystemLibrary.SphereOverlapActors` _returnvalue _searchradius (`|MakeArray` "ObjectTypeQuery1" "ObjectTypeQuery2" "ObjectTypeQuery4" :!type "EObjectTypeQuery Enum") "/Game/BP/Box/BP_Box.BP_Box_C"))
  (bind _box (`self.TouchBox` _outactors))
  (bind _asbp_box (cast `/Game/BP/Box/BP_Box` _box))
  (set `self.BP_Box` _asbp_box)
  (`KismetSystemLibrary.K2_ClearAndInvalidateTimerHandle` (`self.StateTimerHandle`))
  (`self.EnterState_MovingToTarget`))

(event `EnterState_MovingToTarget`
  (bind _returnvalue_location (`KismetMathLibrary.BreakTransform` (`SceneComponent.K2_GetComponentToWorld` (`self.DropPos`))))
  (bind _returnvalue (`self.K2_GetActorLocation` (`self.BP_Box`)))
  ; Moving To Target State
  (set `self.CurrentArmState` "NewEnumerator2")
  (if (`KismetSystemLibrary.IsValid` (`self.ControlRig`))
    (`ControlRigComponent.SetControlTransform` (`self.ControlRig`) (`self.Robot1_End`) (`KismetMathLibrary.Conv_VectorToTransform` _returnvalue) "WorldSpace")
    (if (<= (`KismetMathLibrary.Vector_Distance` (.location (`ControlRigComponent.GetControlTransform` (`self.ControlRig`) (`self.Robot1_End`) "WorldSpace")) _returnvalue) (`self.ReachTolerance`))
      (if (!= _returnvalue_location _returnvalue)
        _))
    (else
      (`KismetSystemLibrary.PrintString` "ERROR : Control Rig Component not Valid")
      (`self.EnterState_SearchingBox`))))

(event `EnterState_PickUpBox`
  (bind _bp_box (`self.BP_Box`))
  ; PicUpBox State
  (set `self.CurrentArmState` "NewEnumerator3")
  (`KismetSystemLibrary.PrintString` "PICK ME PICK ME")
  (if (`KismetSystemLibrary.IsValid` (`self.BP_Box`))
    (`self.K2_AttachToComponent` _bp_box (`self.SkeletalMesh`) (`self.SocketName`) "SnapToTarget" "SnapToTarget" "KeepWorld" true)
    (set `/Game/BP/Box/BP_Box.bSplineMovementAcive` false _bp_box)
    (`ControlRigComponent.SetControlTransform` (`self.ControlRig`) (`self.Robot1_End`) (`SceneComponent.K2_GetComponentToWorld` (`self.DropPos`)) "WorldSpace")
    (else
      (`self.EnterState_SearchingBox`))))

(event `Enter_StateDroppingBox`
  ; Dropping Box State
  (set `self.CurrentArmState` "NewEnumerator5")
  (`KismetSystemLibrary.PrintString` "Drop Box!!")
  (if (`KismetSystemLibrary.IsValid` (`self.BP_Box`))
    (`self.K2_DetachFromActor` (`self.BP_Box`) "KeepWorld" "KeepWorld" "KeepWorld")
    (`PrimitiveComponent.SetSimulatePhysics` (`/Game/BP/Box/BP_Box.StaticMesh` (`self.BP_Box`)) false)
    (`KismetSystemLibrary.PrintString` "Robto Arm : Box Dropped")
    (`KismetArrayLibrary.Array_AddUnique` (`Actor.Tags` (`self.BP_Box`)) (`KismetStringLibrary.Conv_StringToName` (`KismetSystemLibrary.GetObjectName` self)))
    (set `self.BP_Box` null)
    (`self.EnterState_SearchingBox`)
    (else
      (`KismetSystemLibrary.PrintString` "Robot Arm : No Box To Drop, Re-Searching")
      (`self.EnterState_SearchingBox`))))

(fn `TouchBox`
  (params (Actors :type "Array of Actor Object Reference"))
  (returns (Box :type "Actor Object Reference"))
  (locals (FoundBox :type "Actor Object Reference"))
  (for _array_element Actors
    (bind _asbp_box (cast `/Game/BP/Box/BP_Box` _array_element))
    (if true
      (set `local.FoundBox` _asbp_box)
      (break)))
  (return (`local.FoundBox`)))

(fn `UserConstructionScript`)